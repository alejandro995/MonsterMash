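; BP_SM_Carlota is a player-controlled character that moves on world axes and shoves nearby AI characters.
; Enhanced Input mapping is added after BeginPlay, and movement records Directionality and held state, which IsStuck compares against velocity.
; Push sphere-traces for pawns, retags an AI-tagged PaperZD hit as Pushing, launches it away and plays a throttled sound.
; A delayed check on Tick clears the Pushing flag.
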(event Input|EnhancedActionEvents|EnhancedInputActionIA_Move
  (params (ActionValue :type Vector%202D%20Structure) (ElapsedSeconds :type Float%20%28double-precision%29) (TriggeredSeconds :type Float%20%28double-precision%29) (InputAction :type Input%20Action%20Object%20Reference :default "/Game/Blueprints/Input/IA_Move.IA_Move"))
  (:Triggered
    (Pawn|Input|AddMovementInput "1.000000,0.000000,0.000000" (.x ActionValue) false)
    (Pawn|Input|AddMovementInput "0.000000,-1.000000,0.000000" (.y ActionValue) false)
    (Variables|Default|SetDirectionality (Math|Vector2D|MakeVector2D (.x ActionValue) (.y ActionValue))))
  (:Started
    (Variables|Default|SetISHoldingMove true))
  (:Completed
    (Variables|Default|SetISHoldingMove false)))

(event Input|EnhancedActionEvents|EnhancedInputActionIA_Push
  (params (ActionValue :type Boolean) (ElapsedSeconds :type Float%20%28double-precision%29) (TriggeredSeconds :type Float%20%28double-precision%29) (InputAction :type Input%20Action%20Object%20Reference :default "/Game/Blueprints/Input/IA_Push.IA_Push"))
  (bind _capsulecomponent (Variables|Default|GetCapsuleComponent))
  (bind _returnvalue (Transformation|GetWorldLocation _capsulecomponent))
  (:Triggered
    (Variables|Default|SetPushing true)
    (bind (_outhit _returnvalue_2) (Collision|SphereTraceForObjects _returnvalue _returnvalue 6e+01 (Utilities|Array|MakeArray "ObjectTypeQuery3") false 0 "None"))
    (if _returnvalue_2
      (Variables|Default|SetHit%20Actor (.HitActor (Collision|BreakHitResult _outhit)))
      (if (Actor|ActorHasTag (Variables|Default|GetHit%20Actor) "AI")
        (bind _aspaper_zdcharacter (Utilities|Casting|CastToPaperZDCharacter (Variables|Default|GetHit%20Actor)))
        (Variables|/Script/Engine.Actor|SetTags (Variables|Default|GetHit%20Actor) (Utilities|Array|MakeArray "AI" "Pushing"))
        (Character|LaunchCharacter _aspaper_zdcharacter (Math|Vector|MakeVector (* (.x (- (Transformation|GetActorLocation (Variables|Default|GetHit%20Actor)) (.TraceStart (Collision|BreakHitResult _outhit)))) 2e+01) (* (.y (- (Transformation|GetActorLocation (Variables|Default|GetHit%20Actor)) (.TraceStart (Collision|BreakHitResult _outhit)))) 2e+01) 1e+01) false false)
        (if (Variables|Default|Getcan%20sound%20Play)
          (Audio|PlaySound2D "/Game/Sound/RandomSka1.RandomSka1" 1.0 1.0 0.0 0 0)
          (Variables|Default|Setcan%20sound%20Play false)
          (Utilities|FlowControl|Delay 0.2)
          (Variables|Default|Setcan%20sound%20Play true))))))

(event EventBeginPlay
  (Utilities|FlowControl|Delay 0.2)
  (bind _asplayer_controller (Utilities|Casting|CastToPlayerController (Pawn|GetController)))
  (Input|AddMappingContext (PlayerController|LocalPlayerSubsystems|GetEnhancedInputLocalPlayerSubsystem _asplayer_controller) "/Game/Blueprints/Input/IMC_MonsterMash.IMC_MonsterMash" 0 "(bIgnoreAllPressedKeysUntilRelease=True,bForceImmediately=False)"))

(event Collision|EventActorBeginOverlap
  (params (OtherActor :type Actor%20Object%20Reference)))

(event EventTick
  (params (DeltaSeconds :type Float%20%28single-precision%29))
  (Utilities|FlowControl|Delay 0.5)
  (if (Variables|Default|GetPushing)
    (Variables|Default|SetPushing false)))

(fn ConstructionScript)

(fn IsStuck
  (return (and (Variables|Default|GetISHoldingMove) (< (Math|Vector|VectorLength (Transformation|GetVelocity)) (Variables|Default|GetStuckThresHold)))))
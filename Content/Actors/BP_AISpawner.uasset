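; AI spawner actor that fills the level with enemies for each round of the GS_MM game state.
; It spawns after a short delay on BeginPlay and again whenever the EnemyResetSpawner event fires.
; The current round sets the GS_MM enemy count, with round 1 using EnemiesRound3 and round 3 using EnemiesRound1.
; Each enemy is randomly Carlota, Hernando or Pako, placed within a hard-coded X/Y range at fixed height.
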(event Custom|SpawnEnemies
  (Utilities|FlowControl|Delay 1.5)
  (bind _asgs_mm (Utilities|Casting|CastToGS_MM (Game|GetGameState)))
  (switch int (Variables|/Game/GameMode/GS_MM.GS_MM_C|GetRounds _asgs_mm)
    (:1
      (Variables|/Game/GameMode/GS_MM.GS_MM_C|SetEnemies _asgs_mm (Variables|Default|GetEnemiesRound3)))
    (:2
      (Variables|/Game/GameMode/GS_MM.GS_MM_C|SetEnemies _asgs_mm (Variables|Default|GetEnemiesRound2)))
    (:3
      (Variables|/Game/GameMode/GS_MM.GS_MM_C|SetEnemies _asgs_mm (Variables|Default|GetEnemiesRound1))))
  (for _index (range 0 (Variables|/Game/GameMode/GS_MM.GS_MM_C|GetEnemies _asgs_mm))
    (Game|SpawnActorfromClass (Utilities|Select :Index (Math|Random|RandomIntegerinRange 0 2) :Option%200 "/Game/AI/BP_AI_Carlota.BP_AI_Carlota_C" :Option%201 "/Game/AI/BP_AI_Hernando.BP_AI_Hernando_C" :Option%202 "/Game/AI/BP_AI_Pako.BP_AI_Pako_C") (Math|Transform|MakeTransform (Math|Vector|MakeVector (Math|Random|RandomFloatinRange -6e+02 3e+02) (Math|Random|RandomFloatinRange -4e+02 4e+02) 135.0) "0, 0, 0" "1.000000,1.000000,1.000000") "Undefined" "MultiplyWithRoot" 0 0)))

(event EventBeginPlay
  (EventDispatchers|BindEventtoEnemyResetSpawner (delegate Custom|SpawnEnemies))
  (Utilities|FlowControl|Delay 1.5)
  (CallFunction|SpawnEnemies))

(fn ConstructionScript)
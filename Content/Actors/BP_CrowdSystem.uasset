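; BP_CrowdSystem is an actor that lines a spline with animated 2D sprites to form a crowd.
; Its construction script divides the spline length by Spacing and adds a manually attached Paper Flipbook component at each interval, using the spline's world-space location with zero rotation.
; Each component gets a flipbook picked at random from six variables, so the mix is re-rolled whenever construction reruns.
; The event graph has no runtime logic.
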(event EventBeginPlay)

(event Collision|EventActorBeginOverlap
  (params (OtherActor :type Actor%20Object%20Reference)))

(event EventTick
  (params (DeltaSeconds :type Float%20%28single-precision%29)))

(fn ConstructionScript
  (bind _spline (Variables|Default|GetSpline))
  (bind _spacing (Variables|Default|GetSpacing))
  (for _index (range 0 (Math|Float|Truncate (Math|Float|SafeDivide (Spline|GetSplineLength _spline) _spacing)))
    (bind _returnvalue (AddComponent|AddPaperFlipbookComponent true (Math|Transform|MakeTransform (Spline|GetLocationatDistanceAlongSpline _spline (* _index _spacing) "World"))))
    (Sprite|SetFlipbook _returnvalue (.OutItem (Utilities|Array|Random (Utilities|Array|MakeArray (Variables|Default|GetFlipBook) (Variables|Default|GetFlipBook_0) (Variables|Default|GetFlipBook_1) (Variables|Default|GetFlipBook_2) (Variables|Default|GetFlipBook_3) (Variables|Default|GetFlipBook_4)))))))